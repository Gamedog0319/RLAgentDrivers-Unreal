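; BP_RLTrainingManager sets up and runs reinforcement learning training with the Learning Agents plugin.
; On BeginPlay it initializes the interactor, then the policy from that interactor and a neural network data asset, then the trainer from both.
; Every Tick it calls RunTraining with training, game, path and critic settings, without reinitializing the policy or critic networks.
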(event EventBeginPlay
  (Utilities|FlowControl|Sequence
    (:then_0
      (Class|LearningAgentsInteractor|SetupInteractor (Variables|Default|GetBP_RLInteractor)))
    (:then_1
      (Class|LearningAgentsPolicy|SetupPolicy (Variables|Default|GetBP_RLPolicy) (Variables|Default|GetBP_RLInteractor) (Variables|Default|GetPolicy%20Settings) "/Game/LearningAgents/DA_NeuralNetwork.DA_NeuralNetwork"))
    (:then_2
      (Class|LearningAgentsTrainer|SetupTrainer (Variables|Default|GetBP_RLTrainer) (Variables|Default|GetBP_RLInteractor) (Variables|Default|GetBP_RLPolicy) 0 (Variables|Default|GetTrainer%20Settings)))))

(event EventTick
  (params (DeltaSeconds :type Float%20%28single-precision%29))
  (Class|LearningAgentsTrainer|RunTraining (Variables|Default|GetBP_RLTrainer) (Variables|Default|GetTrainer%20Training%20Settings) (Variables|Default|GetTrainer%20Game%20Settings) (Variables|Default|GetTrainer%20Path%20Settings) (Variables|Default|GetCritic%20Settings) false false true))

(fn ConstructionScript)